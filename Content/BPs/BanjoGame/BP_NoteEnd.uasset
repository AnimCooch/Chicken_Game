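; BP_NoteEnd is an actor in the banjo game that displays a colored sphere which can glow on demand, apparently marking the end of a note.
; Its construction script creates a dynamic instance of M_NoteEnd, applies it to the sphere and sets its color from LColor.
; Lightup and Delight switch the glow on and off through the material's GlowIntensity parameter; the event graph holds no logic.
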(event `self.ReceiveBeginPlay`)

(fn `Delight`
  (`MaterialInstanceDynamic.SetScalarParameterValue` (`self.DynamicMaterial`) "GlowIntensity" 0.0))

(fn `Lightup`
  (`MaterialInstanceDynamic.SetScalarParameterValue` (`self.DynamicMaterial`) "GlowIntensity" 50.0))

(fn `UserConstructionScript`
  (bind _returnvalue (`KismetMaterialLibrary.CreateDynamicMaterialInstance` "/Game/BPs/BanjoGame/M_NoteEnd.M_NoteEnd"))
  (bind _output_get (set `self.DynamicMaterial` _returnvalue))
  (`PrimitiveComponent.SetMaterial` (`self.Sphere`) 0 _output_get)
  (`MaterialInstanceDynamic.SetVectorParameterValue` _output_get "Color" (`self.LColor`)))