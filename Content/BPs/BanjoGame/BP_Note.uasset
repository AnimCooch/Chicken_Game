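; BP_Note is a note actor for a banjo game that travels to an endpoint and plays a guitar slap sound on arrival.
; Construction gives the start and end pieces a shared dynamic material, initially black.
; StartMoving applies glow and color, reveals an end piece offset by Length for long notes, then moves the root over a fixed time.
; Tick checks X distance to the endpoint, destroying the note within a threshold.
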(event `StartMoving`
  (bind _endnote (`self.EndNote`))
  (`self.UpdateMaterial`)
  (if (`self.LongNote`)
    (`SceneComponent.SetVisibility` _endnote true false)
    (`SceneComponent.K2_AddLocalOffset` _endnote (`KismetMathLibrary.MakeVector` (`self.Length`)) false false))
  (`KismetSystemLibrary.MoveComponentTo` (`self.DefaultSceneRoot`) (`self.Endpoint`) (struct) false false 3.0))

(event `self.ReceiveTick`
  (params (DeltaSeconds :type "Float (single-precision)"))
  (bind _returnvalue_x (`KismetMathLibrary.BreakVector` (`self.K2_GetActorLocation`)))
  (bind _endpoint_x (`KismetMathLibrary.BreakVector` (`self.Endpoint`)))
  (if (<= (- _returnvalue_x _endpoint_x) 250.0)
    (`GameplayStatics.PlaySound2D` "/Game/SoundEffects/BanjoGame/SC_GuitarSlap.SC_GuitarSlap" 1.0 1.0 0.0 null null)
    (`self.K2_DestroyActor`)))

(fn `UpdateMaterial`
  (bind _dynamicmaterial (`self.DynamicMaterial`))
  (`MaterialInstanceDynamic.SetScalarParameterValue` _dynamicmaterial "GlowIntensity" 10.0)
  (`MaterialInstanceDynamic.SetVectorParameterValue` _dynamicmaterial "Color" (`self.LColor`)))

(fn `UserConstructionScript`
  (bind _returnvalue (`KismetMaterialLibrary.CreateDynamicMaterialInstance` "/Game/BPs/BanjoGame/M_NoteEnd.M_NoteEnd"))
  (bind _output_get (set `self.DynamicMaterial` _returnvalue))
  (`PrimitiveComponent.SetMaterial` (`self.StartNote`) 0 _output_get)
  (`PrimitiveComponent.SetMaterial` (`self.EndNote`) 0 _output_get)
  (`MaterialInstanceDynamic.SetVectorParameterValue` :`self` _output_get :`ParameterName` "Color"))