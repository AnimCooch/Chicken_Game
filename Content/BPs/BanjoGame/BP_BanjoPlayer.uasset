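; BP_BanjoPlayer is the player for the banjo rhythm game, forwarding directional input to the song manager as colored note hits.
; On BeginPlay it adds the IMC_Banjo Enhanced Input mapping context and caches the BP_SongManager found in the level.
; Left, Right, Up and Down map to Red, Yellow, Green and Blue, calling CheckNote on press and DeactivateNote on release.
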(event `self.ReceiveBeginPlay`
  (bind _asplayer_controller (cast `PlayerController` (`self.GetController`)))
  (`/Engine/EditorBlueprintResources/StandardMacros.IsValid` _asplayer_controller
    (:`Is Valid`
      (`EnhancedInputSubsystemInterface.AddMappingContext` (pcsubsystem `EnhancedInputLocalPlayerSubsystem` _asplayer_controller) "/Game/Inputs/Banjo/IMC_Banjo.IMC_Banjo" 0 (struct))
      (bind _outactors (`GameplayStatics.GetAllActorsOfClass` "/Game/BPs/BanjoGame/BP_SongManager.BP_SongManager_C"))
      (for _array_element _outactors
        (set `self.SongManager` _array_element)))))

(event `EnhancedInput|/Game/Inputs/Banjo/IA_Left`
  (params (ActionValue :type Boolean) (ElapsedSeconds :type "Float (double-precision)") (TriggeredSeconds :type "Float (double-precision)") (InputAction :type "InputAction Object Reference" :default "/Game/Inputs/Banjo/IA_Left.IA_Left"))
  (bind _songmanager (`self.SongManager`))
  (:`Started`
    (`/Game/BPs/BanjoGame/BP_SongManager.CheckNote` _songmanager "Red"))
  (:`Completed`
    (`/Game/BPs/BanjoGame/BP_SongManager.DeactivateNote` _songmanager "Red")))

(event `EnhancedInput|/Game/Inputs/Banjo/IA_Right`
  (params (ActionValue :type Boolean) (ElapsedSeconds :type "Float (double-precision)") (TriggeredSeconds :type "Float (double-precision)") (InputAction :type "InputAction Object Reference" :default "/Game/Inputs/Banjo/IA_Right.IA_Right"))
  (bind _songmanager (`self.SongManager`))
  (:`Started`
    (`/Game/BPs/BanjoGame/BP_SongManager.CheckNote` _songmanager "Yellow"))
  (:`Completed`
    (`/Game/BPs/BanjoGame/BP_SongManager.DeactivateNote` _songmanager "Yellow")))

(event `EnhancedInput|/Game/Inputs/Banjo/IA_Up`
  (params (ActionValue :type Boolean) (ElapsedSeconds :type "Float (double-precision)") (TriggeredSeconds :type "Float (double-precision)") (InputAction :type "InputAction Object Reference" :default "/Game/Inputs/Banjo/IA_Up.IA_Up"))
  (bind _songmanager (`self.SongManager`))
  (:`Started`
    (`/Game/BPs/BanjoGame/BP_SongManager.CheckNote` _songmanager "Green"))
  (:`Completed`
    (`/Game/BPs/BanjoGame/BP_SongManager.DeactivateNote` _songmanager "Green")))

(event `EnhancedInput|/Game/Inputs/Banjo/IA_Down`
  (params (ActionValue :type Boolean) (ElapsedSeconds :type "Float (double-precision)") (TriggeredSeconds :type "Float (double-precision)") (InputAction :type "InputAction Object Reference" :default "/Game/Inputs/Banjo/IA_Down.IA_Down"))
  (bind _songmanager (`self.SongManager`))
  (:`Started`
    (`/Game/BPs/BanjoGame/BP_SongManager.CheckNote` _songmanager "Blue"))
  (:`Completed`
    (`/Game/BPs/BanjoGame/BP_SongManager.DeactivateNote` _songmanager "Blue")))

(fn `UserConstructionScript`)