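; Song manager for the banjo rhythm minigame: plays the guitar track, spawns notes and calls Win on BP_BanjoGame after a fixed delay matching the song.
; BeginPlay maps spawn and end actors by color; SpawnNote launches BP_Note between them.
; A looping timer picks random colors, while timeline-driven charting sits unused.
; CheckNote lights the endpoint and destroys a matching note within range; DeactivateNote unlights it.
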(event `StopSong`
  (`AudioComponent.Stop` (`self.SongReference`)))

(event `RandomNote`
  (`self.SpawnNote` (`KismetArrayLibrary.Array_Random` (`self.PossibleColors`))))

(event `PlaySong`
  (bind _returnvalue (`GameplayStatics.CreateSound2D` "/Game/SoundEffects/Music/Guitar_Song_Cue.Guitar_Song_Cue" 1.0 1.0 0.0 null))
  (bind _output_get (set `self.SongReference` _returnvalue))
  (`AudioComponent.Play` _output_get 0.0)
  (`self.SpawningNotes`)
  (`KismetSystemLibrary.Delay` 28.290613)
  (`KismetSystemLibrary.K2_ClearAndInvalidateTimerHandle` (stale `SpawningNotes` _returnvalue))
  (bind _asbp_banjo_game (cast `/Game/BPs/Gamemodes/BP_BanjoGame` (`GameplayStatics.GetGameMode`)))
  (`/Game/BPs/Gamemodes/BP_BanjoGame.Win` _asbp_banjo_game))

(event `SpawningNotes`
  (bind _returnvalue (`KismetSystemLibrary.K2_SetTimerDelegate` (delegate `RandomNote`) 0.5 true)))

(event `StartGame`
  (`self.PlaySong`))

(event `self.ReceiveBeginPlay`
  (bind _outactors (`GameplayStatics.GetAllActorsOfClass` "/Game/BPs/BanjoGame/BP_NoteSpawn.BP_NoteSpawn_C"))
  (for _array_element _outactors
    (`BlueprintMapLibrary.Map_Add` (`self.StartPoints`) (`/Game/BPs/BanjoGame/BP_NoteSpawn.Color` _array_element) _array_element)
    (bind _outactors_2 (`GameplayStatics.GetAllActorsOfClass` "/Game/BPs/BanjoGame/BP_NoteEnd.BP_NoteEnd_C"))
    (for _array_element_2 _outactors_2
      (`BlueprintMapLibrary.Map_Add` (`self.EndPoints`) (`/Game/BPs/BanjoGame/BP_NoteEnd.Color` _array_element_2) _array_element_2))))

(fn `CheckNote`
  (params (NoteColor :type String))
  (locals (NoteHit :type Boolean))
  (bind _value (`BlueprintMapLibrary.Map_Find` (`self.EndPoints`) NoteColor))
  (`/Game/BPs/BanjoGame/BP_NoteEnd.Lightup` _value)
  (bind _outactors (`GameplayStatics.GetAllActorsOfClass` "/Game/BPs/BanjoGame/BP_Note.BP_Note_C"))
  (for _array_element _outactors
    (if (`KismetStringLibrary.EqualEqual_StrStr` (`/Game/BPs/BanjoGame/BP_Note.Color` _array_element) NoteColor)
      (if (<= (`KismetMathLibrary.Vector_Distance` (`self.K2_GetActorLocation` _array_element) (`self.K2_GetActorLocation` _value)) 40.0)
        (set `local.NoteHit` true)
        (`self.K2_DestroyActor` _array_element)
        (break))))
  (if (`local.NoteHit`)
    _))

(fn `DeactivateNote`
  (params (Color :type String))
  (`/Game/BPs/BanjoGame/BP_NoteEnd.Delight` (`BlueprintMapLibrary.Map_Find` (`self.EndPoints`) Color)))

(fn `SpawnNote`
  (params (Color :type String))
  (bind _value (`BlueprintMapLibrary.Map_Find` (`self.EndPoints`) Color))
  (bind (_returnvalue_x _returnvalue_y _returnvalue_z) (`KismetMathLibrary.BreakVector` (`self.K2_GetActorLocation` _value)))
  (bind _returnvalue (`|SpawnActorFromClass` "/Game/BPs/BanjoGame/BP_Note.BP_Note_C" (`KismetMathLibrary.MakeTransform` (`self.K2_GetActorLocation` (`BlueprintMapLibrary.Map_Find` (`self.StartPoints`) Color))) "Undefined" "MultiplyWithRoot" null null))
  (set `/Game/BPs/BanjoGame/BP_Note.LongNote` false _returnvalue)
  (set `/Game/BPs/BanjoGame/BP_Note.Length` 500.0 _returnvalue)
  (set `/Game/BPs/BanjoGame/BP_Note.Endpoint` (`KismetMathLibrary.MakeVector` (- _returnvalue_x 300.0) _returnvalue_y _returnvalue_z) _returnvalue)
  (set `/Game/BPs/BanjoGame/BP_Note.Color` Color _returnvalue)
  (set `/Game/BPs/BanjoGame/BP_Note.LColor` (`/Game/BPs/BanjoGame/BP_NoteEnd.LColor` _value) _returnvalue)
  (`/Game/BPs/BanjoGame/BP_Note.StartMoving` _returnvalue))

(fn `UserConstructionScript`
  (locals (NewLocalVar :type "Map of Float (double-precision) to  Structure") (NewLocalVar_0 :type "Map of Float (double-precision) to  Structure") (NewLocalVar_1 :type "Map of Float (double-precision) to  Structure") (NewLocalVar_2 :type "Map of Float (double-precision) to  Structure") (NewLocalVar_3 :type "Map of Float (double-precision) to  Structure")))