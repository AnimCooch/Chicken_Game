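; BP_Farmer2 is a boss fight farmer actor whose skeletal mesh slowly turns to face the player.
; Each tick, it computes a look-at rotation to the player pawn, offsets yaw by -90 degrees and eases toward it with RInterpTo, keeping only yaw.
; A similar node that would pitch the Arrow component is left unconnected, and the blueprint contains no attack or other behavior.
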(event `self.ReceiveTick`
  (params (DeltaSeconds :type "Float (single-precision)"))
  (bind _skeletalmesh (`self.SkeletalMesh`))
  (bind (_returnvalue_roll _returnvalue_pitch _returnvalue_yaw) (`KismetMathLibrary.BreakRotator` (`KismetMathLibrary.FindLookAtRotation` (`SceneComponent.K2_GetComponentLocation` _skeletalmesh) (`self.K2_GetActorLocation` (`GameplayStatics.GetPlayerPawn` 0)))))
  (bind (_returnvalue_roll_2 _returnvalue_pitch_2 _returnvalue_yaw_2) (`KismetMathLibrary.BreakRotator` (`KismetMathLibrary.RInterpTo` (`SceneComponent.K2_GetComponentRotation` _skeletalmesh) (`KismetMathLibrary.MakeRotator` _returnvalue_roll _returnvalue_pitch (- _returnvalue_yaw 90.0)) DeltaSeconds 1.0)))
  (`SceneComponent.K2_SetWorldRotation` _skeletalmesh (`KismetMathLibrary.MakeRotator` 0.0 0.0 _returnvalue_yaw_2) false false))

(fn `UserConstructionScript`)