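; BP_PlayerTrack is a boss fight actor that builds a circular spline track, presumably for player movement, with no active gameplay logic of its own.
; The construction script clears the Track spline and places four local-space points at SplineRadius along the positive and negative X and Y axes.
; It then sets perpendicular tangents scaled from the radius to approximate a circle, so changing SplineRadius resizes the ring.
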(fn `UserConstructionScript`
  (locals (SplineNum :type Integer))
  (bind _track (`self.Track`))
  (bind _splineradius (`self.SplineRadius`))
  (bind _splinenum (`local.SplineNum`))
  (bind _splinenum_2 (`local.SplineNum`))
  (bind _splinenum_3 (`local.SplineNum`))
  (bind _splinenum_4 (`local.SplineNum`))
  (bind _returnvalue (* _splineradius -1.0))
  (`SplineComponent.ClearSplinePoints` _track true)
  (`SplineComponent.AddSplinePoint` _track (`KismetMathLibrary.MakeVector` _splineradius) "Local" true)
  (`SplineComponent.AddSplinePoint` _track (`KismetMathLibrary.MakeVector` 0.0 _splineradius) "Local" true)
  (`SplineComponent.AddSplinePoint` _track (`KismetMathLibrary.MakeVector` _returnvalue) "Local" true)
  (`SplineComponent.AddSplinePoint` _track (`KismetMathLibrary.MakeVector` 0.0 _returnvalue) "Local" true)
  (for _index (range (+ (`SplineComponent.GetNumberOfSplinePoints` (`self.Track`)) 1))
    (set `local.SplineNum` _index)
    (if (== _splinenum_4 0)
      (`SplineComponent.SetTangentAtSplinePoint` (`self.Track`) _splinenum_4 (`KismetMathLibrary.MakeVector` 0.0 (* (* (`self.SplineRadius`) 1.5) 1.0)) "Local" true)
      (elif (== _splinenum 1)
        (`SplineComponent.SetTangentAtSplinePoint` (`self.Track`) _splinenum (`KismetMathLibrary.MakeVector` (* (* (`self.SplineRadius`) 1.5) -1.0)) "Local" true)
        (elif (== _splinenum_2 2)
          (`SplineComponent.SetTangentAtSplinePoint` (`self.Track`) _splinenum_2 (`KismetMathLibrary.MakeVector` 0.0 (* (* (`self.SplineRadius`) 1.5) -1.0)) "Local" true)
          (elif (== _splinenum_3 3)
            (`SplineComponent.SetTangentAtSplinePoint` (`self.Track`) _splinenum_3 (`KismetMathLibrary.MakeVector` (* (* (`self.SplineRadius`) 1.5) 1.0)) "Local" true)))))))