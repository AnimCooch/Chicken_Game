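; BP_FarmerBoss is the farmer boss, which turns its body and pitches its gun toward the player every tick.
; A randomized cooldown triggers either a randomly spread shotgun burst or, more often, a full ring of BP_Projectiles, telegraphed by a brief rage-material swap.
; Original materials are cached in the Construction Script for restoring afterward.
; Hurt lowers health, updates the FarmerHealth widget and calls Win on the BP_BossFight game mode at zero.
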(event `self.ReceiveTick`
  (params (DeltaSeconds :type "Float (single-precision)"))
  (bind _gun (`self.Gun`))
  (bind _capsulecomponent (`self.CapsuleComponent`))
  (bind (_returnvalue_roll _returnvalue_pitch _returnvalue_yaw) (`KismetMathLibrary.BreakRotator` (`SceneComponent.K2_GetComponentRotation` (`self.Gun`))))
  (bind (_returnvalue_x _returnvalue_y _returnvalue_z) (`KismetMathLibrary.BreakVector` (`self.K2_GetActorLocation` (`GameplayStatics.GetPlayerPawn` 0))))
  (bind (_returnvalue_roll_2 _returnvalue_pitch_2 _returnvalue_yaw_2) (`KismetMathLibrary.BreakRotator` (`KismetMathLibrary.FindLookAtRotation` (`SceneComponent.K2_GetComponentLocation` _capsulecomponent) (`self.K2_GetActorLocation` (`GameplayStatics.GetPlayerPawn` 0)))))
  (bind (_returnvalue_roll_3 _returnvalue_pitch_3) (`KismetMathLibrary.BreakRotator` (`KismetMathLibrary.RInterpTo` (`SceneComponent.K2_GetComponentRotation` _gun) (`KismetMathLibrary.FindLookAtRotation` (`SceneComponent.K2_GetComponentLocation` _gun) (`KismetMathLibrary.MakeVector` _returnvalue_x _returnvalue_y (+ _returnvalue_z 50.0))) DeltaSeconds 15.0)))
  (bind (_returnvalue_roll_4 _returnvalue_pitch_4 _returnvalue_yaw_3) (`KismetMathLibrary.BreakRotator` (`KismetMathLibrary.RInterpTo` (`SceneComponent.K2_GetComponentRotation` _capsulecomponent) (`KismetMathLibrary.MakeRotator` _returnvalue_roll_2 _returnvalue_pitch_2 (- _returnvalue_yaw_2 0.0)) DeltaSeconds 15.0)))
  (`self.Attacking` DeltaSeconds)
  (`SceneComponent.K2_SetWorldRotation` _capsulecomponent (`KismetMathLibrary.MakeRotator` 0.0 0.0 _returnvalue_yaw_3) false false)
  (`SceneComponent.K2_SetWorldRotation` (`self.Gun`) (`KismetMathLibrary.MakeRotator` _returnvalue_roll _returnvalue_pitch_3 _returnvalue_yaw) false false))

(event `Attacking`
  (params (Deltatime :type "Float (double-precision)"))
  (if (not (`self.isAttacking`))
    (bind _output_get (set `self.AttackCoolDown` (- (`self.AttackCoolDown`) Deltatime)))
    (if (<= _output_get 0.0)
      (set `self.isAttacking` true)
      (set `self.AttackCoolDown` (`KismetMathLibrary.RandomFloatInRange` 3.0 5.0))
      (`self.Shoot`))))

(event `Shoot`
  (bind _returnvalue (`SceneComponent.K2_GetComponentToWorld` (`self.Gun`)))
  (if (> (`KismetMathLibrary.RandomFloatInRange` 1.0 5.0) 4.0)
    (`GameplayStatics.PlaySound2D` "/Game/SoundEffects/BossFight/ShotgunShot_Cue.ShotgunShot_Cue" 1.0 1.0 0.0 null null)
    (for _ (range 10)
      (`|SpawnActorFromClass` "/Game/BPs/BossFight/BP_Projectile.BP_Projectile_C" (`KismetMathLibrary.MakeTransform` (.location _returnvalue) (`KismetMathLibrary.MakeRotator` (+ (.roll (.rotation _returnvalue)) (`KismetMathLibrary.RandomFloatInRange` (* (`self.RandomFireRange`) -1.0) (`self.RandomFireRange`))) (+ (.pitch (.rotation _returnvalue)) (`KismetMathLibrary.RandomFloatInRange` (* (`self.RandomFireRange`) -1.0) (`self.RandomFireRange`))) (+ (.yaw (.rotation _returnvalue)) (`KismetMathLibrary.RandomFloatInRange` (* (`self.RandomFireRange`) -1.0) (`self.RandomFireRange`))))) "Undefined" "MultiplyWithRoot" null null)
      (set `self.isAttacking` false))
    (else
      (`self.RingAttack`))))

(event `self.ReceiveBeginPlay`
  (bind _returnvalue (`|CreateWidget` "/Game/BPs/BossFight/FarmerHealth.FarmerHealth_C"))
  (bind _output_get (set `self.FarmerHealthWidget` _returnvalue))
  (`UserWidget.AddToViewport` _output_get 0))

(event `RingAttack`
  (bind _returnvalue (`SceneComponent.K2_GetComponentToWorld` (`self.CapsuleComponent`)))
  (`self.SetRageMaterials`)
  (`KismetSystemLibrary.Delay` 0.5)
  (`GameplayStatics.PlaySound2D` "/Game/SoundEffects/BossFight/ShotgunShot_Cue.ShotgunShot_Cue" 1.0 1.0 0.0 null null)
  (for _index (range 73)
    (`|SpawnActorFromClass` "/Game/BPs/BossFight/BP_Projectile.BP_Projectile_C" (`KismetMathLibrary.MakeTransform` (`KismetMathLibrary.MakeVector` (.x (.location _returnvalue)) (.y (.location _returnvalue)) (- (.z (.location _returnvalue)) 30.0)) (`KismetMathLibrary.MakeRotator` 0.0 0.0 (+ (.yaw (.rotation _returnvalue)) (* _index 5)))) "AlwaysSpawn" "MultiplyWithRoot" null null)
    (`self.ResetMaterials`)
    (set `self.isAttacking` false)))

(event `Hurt`
  (`GameplayStatics.PlaySound2D` "/Game/BPs/BossFight/splat-sound-effect-free-download.splat-sound-effect-free-download" 1.0 1.0 0.0 null null)
  (bind _result (`/Engine/EditorBlueprintResources/StandardMacros.DecrementFloat` (`self.Health`))
    (:`  `
      (set `ProgressBar.Percent` (/ _result (`self.MaxHealth`)) (`/Game/BPs/BossFight/FarmerHealth.ProgressBar_0` (`self.FarmerHealthWidget`)))
      (if (<= (`self.Health`) 0.0)
        (bind _asbp_boss_fight (cast `/Game/BPs/Gamemodes/BP_BossFight` (`GameplayStatics.GetGameMode`)))
        (`/Game/BPs/Gamemodes/BP_BossFight.Win` _asbp_boss_fight)))))

(fn `ResetMaterials`
  (for (_array_element _array_index) (`self.DefaultMaterials`)
    (`PrimitiveComponent.SetMaterial` (`self.Farmer`) _array_index _array_element)))

(fn `SetRageMaterials`
  (bind _farmer (`self.Farmer`))
  (for (_ _array_index) (`MeshComponent.GetMaterials` _farmer)
    (`PrimitiveComponent.SetMaterial` _farmer _array_index "/Game/BPs/BossFight/M_FarmerRage.M_FarmerRage")))

(fn `UserConstructionScript`
  (for _array_element (`MeshComponent.GetMaterials` (`self.Farmer`))
    (`KismetArrayLibrary.Array_Add` (`self.DefaultMaterials`) _array_element)))