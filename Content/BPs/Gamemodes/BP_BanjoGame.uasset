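; Game mode for the banjo chicken minigame, handling strikes, win and loss.
; BeginPlay caches the BP_SongManager, and ShowChicken creates the life widget whose X marks UpdateChicken reveals as PlayerScore rises, losing on the third.
; Both endings pause the game, stop the song, play a sting and show WBP_Lose, which Win relabels as a victory screen.
; Its button reloads L_ChickenGame after a loss or opens L_Hub after a win.
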(event `Restart`
  (`GameplayStatics.OpenLevel` "L_ChickenGame"))

(event `UpdateChicken`
  (bind _returnvalue (`GameplayStatics.GetPlayerController` 0))
  (bind _playerscore (`self.PlayerScore`))
  (if (> _playerscore 0)
    (`Widget.SetVisibility` (`/Game/BPs/BanjoGame/UI/WBP_Life.X1` (`self.LifeWidget`)) "Visible")
    (if (> _playerscore 1)
      (`Widget.SetVisibility` (`/Game/BPs/BanjoGame/UI/WBP_Life.X2` (`self.LifeWidget`)) "Visible")
      (if (> _playerscore 2)
        (`Widget.SetVisibility` (`/Game/BPs/BanjoGame/UI/WBP_Life.X3` (`self.LifeWidget`)) "Visible")
        (`GameplayStatics.SetGamePaused` true)
        (`/Game/BPs/BanjoGame/BP_SongManager.StopSong` (`self.SongManager`))
        (`GameplayStatics.PlaySound2D` "/Game/SoundEffects/Music/Bad_End.Bad_End" 1.0 1.0 0.0 null null)
        (bind _returnvalue_2 (`|CreateWidget` "/Game/BPs/BanjoGame/UI/WBP_Lose.WBP_Lose_C"))
        (bind _output_get (set `self.LoseWidget` _returnvalue_2))
        (`UserWidget.AddToViewport` _output_get 0)
        (add `Button.OnPressed` (`/Game/BPs/BanjoGame/UI/WBP_Lose.RestartButton` (`self.LoseWidget`)) (delegate `Restart`))
        (set `PlayerController.bShowMouseCursor` true _returnvalue)
        (`WidgetBlueprintLibrary.SetInputMode_UIOnlyEx` _returnvalue (`self.LoseWidget`) "LockAlways")))))

(event `ShowChicken`
  (bind _returnvalue (`|CreateWidget` "/Game/BPs/BanjoGame/UI/WBP_Life.WBP_Life_C"))
  (bind _output_get (set `self.LifeWidget` _returnvalue))
  (`UserWidget.AddToViewport` (`self.LifeWidget`) 0)
  (`UserWidget.AddToViewport` _output_get 0))

(event `self.ReceiveBeginPlay`
  (bind _outactors (`GameplayStatics.GetAllActorsOfClass` "/Game/BPs/BanjoGame/BP_SongManager.BP_SongManager_C"))
  (for _array_element _outactors
    (set `self.SongManager` _array_element)))

(event `Win`
  (bind _returnvalue (`GameplayStatics.GetPlayerController` 0))
  (`GameplayStatics.SetGamePaused` true)
  (`/Game/BPs/BanjoGame/BP_SongManager.StopSong` (`self.SongManager`))
  (`GameplayStatics.PlaySound2D` "/Game/SoundEffects/Music/Good_End.Good_End" 1.0 1.0 0.0 null null)
  (bind _returnvalue_2 (`|CreateWidget` "/Game/BPs/BanjoGame/UI/WBP_Lose.WBP_Lose_C"))
  (bind _output_get (set `self.LoseWidget` _returnvalue_2))
  (set `TextBlock.Text` "To Farm" (`/Game/BPs/BanjoGame/UI/WBP_Lose.ButtonText` _output_get))
  (set `TextBlock.Text` "YOU DID IT!" (`/Game/BPs/BanjoGame/UI/WBP_Lose.TextBlock_0` _output_get))
  (`UserWidget.AddToViewport` _output_get 0)
  (add `Button.OnPressed` (`/Game/BPs/BanjoGame/UI/WBP_Lose.RestartButton` (`self.LoseWidget`)) (delegate `GoToHub`))
  (set `PlayerController.bShowMouseCursor` true _returnvalue)
  (`WidgetBlueprintLibrary.SetInputMode_UIOnlyEx` _returnvalue (`self.LoseWidget`) "LockAlways"))

(event `GoToHub`
  (`GameplayStatics.OpenLevel` "L_Hub"))

(fn `UserConstructionScript`)