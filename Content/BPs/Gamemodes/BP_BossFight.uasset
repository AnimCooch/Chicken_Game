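; Game mode for the farmer boss fight that handles music and the win and lose outcomes.
; BeginPlay sets game-only input and starts the fight music.
; Win and Lose each pause the game, swap music for an ending sound and show a mouse-driven WBP_Lose screen, relabeled on a win.
; Its button reloads L_FarmerGame after a loss or opens L_Hub after a win.
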(event `self.ReceiveBeginPlay`
  (`WidgetBlueprintLibrary.SetInputMode_GameOnly` (`GameplayStatics.GetPlayerController` 0))
  (bind _returnvalue (`GameplayStatics.CreateSound2D` "/Game/SoundEffects/Music/Boss_Fight_-_9_14_24__3_24 PM.Boss_Fight_-_9_14_24__3_24 PM" 1.0 1.0 0.0 null))
  (bind _output_get (set `self.BossFightMusic` _returnvalue))
  (`AudioComponent.Play` (`self.BossFightMusic`) 0.0)
  (`AudioComponent.Play` _output_get 0.0))

(event `Lose`
  (bind _returnvalue (`GameplayStatics.GetPlayerController` 0))
  (`GameplayStatics.SetGamePaused` true)
  (`AudioComponent.Stop` (`self.BossFightMusic`))
  (`GameplayStatics.PlaySound2D` "/Game/SoundEffects/Music/Bad_End.Bad_End" 1.0 1.0 0.0 null null)
  (bind _returnvalue_2 (`|CreateWidget` "/Game/BPs/BanjoGame/UI/WBP_Lose.WBP_Lose_C"))
  (bind _output_get (set `self.LoseWidget` _returnvalue_2))
  (`UserWidget.AddToViewport` _output_get 0)
  (set `TextBlock.Text` "THE FARMER LIVES" (`/Game/BPs/BanjoGame/UI/WBP_Lose.TextBlock_0` _output_get))
  (add `Button.OnPressed` (`/Game/BPs/BanjoGame/UI/WBP_Lose.RestartButton` _output_get) (delegate `Restart`))
  (set `PlayerController.bShowMouseCursor` true _returnvalue)
  (`WidgetBlueprintLibrary.SetInputMode_UIOnlyEx` _returnvalue _output_get "LockAlways"))

(event `Restart`
  (`GameplayStatics.OpenLevel` "L_FarmerGame"))

(event `Win`
  (bind _returnvalue (`GameplayStatics.GetPlayerController` 0))
  (`GameplayStatics.SetGamePaused` true)
  (`AudioComponent.Stop` (`self.BossFightMusic`))
  (`GameplayStatics.PlaySound2D` "/Game/SoundEffects/Music/Good_End.Good_End" 1.0 1.0 0.0 null null)
  (bind _returnvalue_2 (`|CreateWidget` "/Game/BPs/BanjoGame/UI/WBP_Lose.WBP_Lose_C"))
  (bind _output_get (set `self.LoseWidget` _returnvalue_2))
  (set `TextBlock.Text` "To Farm" (`/Game/BPs/BanjoGame/UI/WBP_Lose.ButtonText` _output_get))
  (set `TextBlock.Text` "YOU DID IT!" (`/Game/BPs/BanjoGame/UI/WBP_Lose.TextBlock_0` _output_get))
  (`UserWidget.AddToViewport` _output_get 0)
  (add `Button.OnPressed` (`/Game/BPs/BanjoGame/UI/WBP_Lose.RestartButton` (`self.LoseWidget`)) (delegate `GoToHub`))
  (set `PlayerController.bShowMouseCursor` true _returnvalue)
  (`WidgetBlueprintLibrary.SetInputMode_UIOnlyEx` _returnvalue (`self.LoseWidget`) "LockAlways"))

(event `GoToHub`
  (`GameplayStatics.OpenLevel` "L_Hub"))

(fn `UserConstructionScript`)